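; An interactable door actor that swings open and closed when the player interacts with it.
; Each OnInteract toggles IsDoorClosed, plays the same 2D door sound and runs the OpenDoors timeline forward to open or in reverse to close.
; The timeline alpha lerps the Pivot component's relative yaw through a quarter turn.
; IsInteractable always returns true, so the door has no lock or other condition.
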(event `/Game/Blueprints/Interfaces/BPI_Interact.OnInteract`
  (params (`Interactingg Player` :type "Character Object Reference"))
  (if (`self.IsDoorClosed`)
    (set `self.IsDoorClosed` false)
    (`GameplayStatics.PlaySound2D` "/Game/Audio/doorsound2.doorsound2" 1.0 1.0 0.0 null null)
    (bind (_direction _alpha) (`Timeline|OpenDoors` :!label _label)
      (:`Update`
        (`SceneComponent.K2_SetRelativeRotation` (`self.Pivot`) (`KismetMathLibrary.MakeRotator` 0.0 0.0 (`KismetMathLibrary.Lerp` 0.0 -90.0 _alpha)) false false)))
    (else
      (set `self.IsDoorClosed` true)
      (`GameplayStatics.PlaySound2D` "/Game/Audio/doorsound2.doorsound2" 1.0 1.0 0.0 null null)
      (goto _label :!via `Reverse`))))

(fn `IsInteractable`
  (returns (Interactable :type Boolean))
  (return true))

(fn `UserConstructionScript`
  (`parent.UserConstructionScript`))